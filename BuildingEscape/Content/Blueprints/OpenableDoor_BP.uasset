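; Openable door actor that swings around its yaw axis when its OpenDoor component signals open or close.
; On BeginPlay it stores the initial rotation, and the MoveDoor timeline adds an animated angle to it each update.
; A timeline event track plays a door lock sound at the actor's location, and closing reverses the same timeline.
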(event `self.ReceiveBeginPlay`
  (set `self.initialRotation` (`self.K2_GetActorRotation`)))

(event `self.OpenDoor.OnOpen`
  (bind (_direction _openangle) (`Timeline|MoveDoor` :!label _label)
    (:`Update`
      (`self.K2_SetActorRotation` (`KismetMathLibrary.ComposeRotators` (`KismetMathLibrary.MakeRotator` 0.0 0.0 _openangle) (`self.initialRotation`))))
    (:`SoundTiming`
      (`GameplayStatics.PlaySoundAtLocation` "/Game/Audio/door-lock.door-lock" (`self.K2_GetActorLocation`) (struct) 0.5 1.0))))

(event `self.OpenDoor.OnClose`
  (goto _label :!via `Reverse`))

(fn `UserConstructionScript`)